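; MidiListener is a Blueprint that listens to a MIDI device and relays selected controller input through an event dispatcher.
; BeginPlay prints the available devices, and the first Tick creates a controller for the DeviceID variable and binds its MIDI event.
; Events of type 11 (control change) whose ID is in ControlIDs fire MIDIControlEventDispatcher with the array index and velocity, alongside color-coded debug prints.
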(event `self.ReceiveBeginPlay`
  ;[1 1 1] Print MIDI Devices
  (bind _outmididevices (`MIDIDeviceManager.FindMIDIDevices`))
  (for (_array_element _array_index) _outmididevices
    (bind (_deviceid _devicename) (break `FoundMIDIDevice` _array_element))
    (`KismetSystemLibrary.PrintText` (`|FormatText` "{DeviceName} : {DeviceID}" (`KismetTextLibrary.Conv_StringToText` _devicename) (`KismetTextLibrary.Conv_IntToText` _deviceid)) false true (`KismetMathLibrary.LinearColorLerpUsingHSV` (struct :`R` 0.161928 :`G` 0.548735 :`B` 1.0 :`A` 1.0) (struct :`R` 0.416569 :`G` 1.0 :`B` 0.11293 :`A` 1.0) (/ _array_index (`KismetArrayLibrary.Array_Length` _outmididevices))) 20.0)))

(event `self.ReceiveTick`
  (params (DeltaSeconds :type "Float (single-precision)"))
  (bind _device_id (`self.Device ID`))
  ;[1 1 1] Select MIDI Device by Device ID Var
  (`/Engine/EditorBlueprintResources/StandardMacros.DoOnce` false
    (:`Completed`
      (bind _returnvalue (`MIDIDeviceManager.CreateMIDIDeviceController` _device_id))
      (`/Engine/EditorBlueprintResources/StandardMacros.IsValid` _returnvalue
        (:`Is Valid`
          (bind _output_get (set `self.MIDIController` _returnvalue)))
        (:`Is Not Valid`
          _))
      (`KismetSystemLibrary.PrintString` (`KismetStringLibrary.Concat_StrStr` "Current Controller: " (`KismetSystemLibrary.GetDisplayName` _output_get) " | Port " (`KismetStringLibrary.Conv_IntToString` _device_id)) false true (struct :`G` 0.66 :`B` 1.0 :`A` 1.0) 20.0)
      (add `MIDIDeviceController.OnMIDIEvent` _output_get (delegate `MIDIEvent_0`)))))

(event `MIDIEvent_0`
  (params (MIDIDeviceController :type "MIDIDeviceController Object Reference") (Timestamp :type Integer) (EventType :type "EMIDIEventType Enum" :default "Unknown") (Channel :type Integer) (ControlID :type Integer) (Velocity :type Integer) (RawEventType :type Integer))
  ;[1 1 1] MIDIEvent Debug Info
  (`/Engine/EditorBlueprintResources/StandardMacros.IsValid` MIDIDeviceController
    (:`Is Valid`
      (if (!= ControlID 0)
        (`KismetSystemLibrary.PrintText` (`|FormatText` "{Timestamp}: Ch {Channel} - {EventType}/ID: {ControlID}, Vel: {Velocity}" Timestamp Channel (`KismetTextLibrary.Conv_ByteToText` EventType) ControlID Velocity) false true (struct :`R` 1.0 :`G` 0.950883 :`B` 0.066792 :`A` 1.0) 2.0 "RawMIDIData")
        (for (_array_element _array_index) (`self.Control IDs`)
          (if (and (== _array_element ControlID) (== (`KismetMathLibrary.Conv_ByteToInt` EventType) 11))
            (`self.MIDIControlEventDispatcher` _array_index Velocity)
            (`KismetSystemLibrary.PrintText` (`|FormatText` "Index {Index}: Vel {Velocity}" _array_index Velocity) true true (`KismetMathLibrary.LinearColorLerpUsingHSV` (struct :`R` 0.03125 :`G` 0.000683 :`A` 1.0) (struct :`R` 1.0 :`G` 0.119792 :`B` 0.144148 :`A` 1.0) (/ Velocity 127)) 30.0 (`KismetStringLibrary.Conv_StringToName` (`KismetStringLibrary.Concat_StrStr` "MIDIControlIndex" (`KismetStringLibrary.Conv_IntToString` _array_index))))
            (break)))))))