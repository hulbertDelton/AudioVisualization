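; Actor that visualizes audio frequency spectrum magnitudes as a row of FrequencyBouncer cubes.
; On BeginPlay it spawns one FrequencyBouncer child actor per AudioDispatcher spectrum band, spaced evenly along local X, and caches them in an array.
; It then binds to the dispatcher's all-frequency magnitude event and forwards each band's magnitude to the bouncer at the matching index via OnMagnitudeChange.
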(event `DoMagnitude_Event`
  (params (Mags :type "Array of Float (double-precision) (by ref)"))
  (for (_array_element _array_index) (`self.FrequencyCubes`)
    (`/Game/AudioVisualizerContent/Blueprints/FrequencyBouncer.OnMagnitudeChange` _array_element (`|GetArrayItem` Mags _array_index))))

(event `self.ReceiveBeginPlay`
  (for _index (range (`/Game/CodyJunk/AudioAnalyzer.Spectrum Band Count` (`self.AudioDispatcher`)))
    (bind _returnvalue (`AddComponent|NODE_AddChildActorComponent-0` :`RelativeTransform` (`KismetMathLibrary.MakeTransform` (`KismetMathLibrary.MakeVector` (`KismetMathLibrary.Conv_IntToDouble` (* _index 10))) (.rotation (`self.GetTransform`)))))
    (`ChildActorComponent.SetChildActorClass` _returnvalue "/Game/AudioVisualizerContent/Blueprints/FrequencyBouncer.FrequencyBouncer_C")
    (bind _asfrequency_bouncer (cast `/Game/AudioVisualizerContent/Blueprints/FrequencyBouncer` (`ChildActorComponent.ChildActor` _returnvalue)))
    (`KismetArrayLibrary.Array_Add` (`self.FrequencyCubes`) _asfrequency_bouncer))
  (add `/Game/CodyJunk/AudioAnalyzer.OnAllFrequencyMagnitude` (`self.AudioDispatcher`) (delegate `DoMagnitude_Event`)))

(fn `UserConstructionScript`)