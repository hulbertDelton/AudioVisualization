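; Laser light actor for an audio visualizer that swings its light base toward randomized orientations.
; BeginPlay gives LightBase a dynamic M_BlueLight material instance with its LightColor set to white.
; OnTargetRotationChanged picks a random pitch and a wider yaw range scaled from MaxRotation, and Tick rotates LightBase there at constant speed.
; The event's color input is unused, as the recoloring nodes are disconnected.
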(event `self.ReceiveBeginPlay`
  (bind _returnvalue (`PrimitiveComponent.CreateDynamicMaterialInstance` (`self.LightBase`) 0 "/Game/AudioVisualizerContent/ArtAssets/Materials/M_BlueLight.M_BlueLight" "None"))
  (`PrimitiveComponent.SetMaterial` (`self.LightBase`) 0 _returnvalue)
  (`MaterialInstanceDynamic.SetVectorParameterValue` _returnvalue "LightColor" (`KismetMathLibrary.LinearColor_White`)))

(event `OnTargetRotationChanged`
  (params (NewSetColor :type "LinearColor Structure"))
  (bind _maxrotation (`self.MaxRotation`))
  (set `self.TargetRotation` (`KismetMathLibrary.MakeRotator` 0.0 (* (`KismetMathLibrary.RandomFloat`) _maxrotation) (* (* (`KismetMathLibrary.RandomFloat`) _maxrotation) 4.0))))

(event `self.ReceiveTick`
  (params (DeltaSeconds :type "Float (single-precision)"))
  (bind _lightbase (`self.LightBase`))
  (`SceneComponent.K2_SetRelativeRotation` _lightbase (`KismetMathLibrary.RInterpTo_Constant` (`SceneComponent.RelativeRotation` _lightbase) (`self.TargetRotation`) DeltaSeconds 100.0) false false))

(fn `UserConstructionScript`)