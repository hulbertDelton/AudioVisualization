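; FrequencyBouncer is an audio visualizer Blueprint that bounces its Root's Z scale in response to frequency magnitude.
; OnMagnitudeChange compares the raw input to the current Magnitude, and when higher stores it multiplied by a gain and applies it immediately.
; Tick applies Magnitude as Z scale, then decays it at a constant rate toward a small floor.
; BeginPlay saves the initial Z scale in DefaultZ, which the graph never reads.
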(event `OnMagnitudeChange`
  (params (newMagnitude :type "Float (double-precision)"))
  (bind _root (`self.Root`))
  (if (> newMagnitude (`self.Magnitude`))
    (bind _output_get (set `self.Magnitude` (* newMagnitude 10.0)))
    (`SceneComponent.SetRelativeScale3D` _root (`KismetMathLibrary.MakeVector` (.x (`SceneComponent.RelativeScale3D` _root)) (.y (`SceneComponent.RelativeScale3D` _root)) _output_get))))

(event `self.ReceiveBeginPlay`
  (set `self.defaultZ` (.z (`SceneComponent.RelativeScale3D` (`self.Root`)))))

(event `self.ReceiveTick`
  (params (DeltaSeconds :type "Float (single-precision)"))
  (bind _root (`self.Root`))
  (`SceneComponent.SetRelativeScale3D` _root (`KismetMathLibrary.MakeVector` (.x (`SceneComponent.RelativeScale3D` _root)) (.y (`SceneComponent.RelativeScale3D` _root)) (`self.Magnitude`)))
  (set `self.Magnitude` (`KismetMathLibrary.FInterpTo_Constant` (`self.Magnitude`) 0.01 DeltaSeconds 25.0)))

(fn `UserConstructionScript`)