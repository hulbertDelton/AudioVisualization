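; BeachBall is an audio-reactive physics ball for the audio visualizer content, pushed around by the music.
; On BeginPlay it binds to the bass and mids magnitude events of an AudioDispatcher.
; Bass applies an upward impulse scaled by magnitude, while mids apply a random horizontal impulse scaled the same way, so the ball hops and scatters with the sound.
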(event `self.ReceiveBeginPlay`
  (bind _audiodispatcher (`self.AudioDispatcher`))
  (add `/Game/CodyJunk/AudioAnalyzer.OnBassMagnitude` _audiodispatcher (delegate `OnBassTriggered`))
  (add `/Game/CodyJunk/AudioAnalyzer.OnMidsMagnitude` _audiodispatcher (delegate `OnMidsTriggered`)))

(event `OnBassTriggered`
  (params (Magnitude :type "Float (double-precision)"))
  (`PrimitiveComponent.AddImpulse` (`self.Ball`) (`KismetMathLibrary.MakeVector` 0.0 0.0 (* Magnitude 1000.0)) "None" false))

(event `OnMidsTriggered`
  (params (Mag :type "Float (double-precision)"))
  (`PrimitiveComponent.AddImpulse` (`self.Ball`) (`KismetMathLibrary.MakeVector` (* Mag (`KismetMathLibrary.RandomFloatInRange` -2500.0 2500.0)) (* Mag (`KismetMathLibrary.RandomFloatInRange` -2500.0 2500.0))) "None" false))

(fn `UserConstructionScript`)